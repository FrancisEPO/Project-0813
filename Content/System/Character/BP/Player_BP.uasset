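; First-person player character handling Enhanced Input movement, procedural camera effects and a rifle/pistol inventory.
; A state enum sets sprint and crouch speeds, with an overhead box trace gating stand-up.
; Tick drives velocity-based camera shake, interpolated sway and interaction highlight traces; a timer trace auto-focuses depth of field.
; Pickups spawn guns from data assets; swaps lower the arms via timeline and re-socket weapons; firing messages the gun and plays montages.
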(event `self.ReceiveTick`
  (params (DeltaSeconds :type "Float (single-precision)"))
  (bind (_x _y) (`KismetMathLibrary.BreakVector2D` (`self.Action Value`)))
  (`|ExecutionSequence`
    (:`then_0`
      (`self.CameraShake`))
    (:`then_1`
      ;[1 1 1] 在Sway的过程中需要tick更新
      (`self.YawSway` _x)
      (`self.PitchSway` _y)
      (`self.RollSway` _x))
    (:`then_2`
      (`self.SceneInteractionLineDetection`))))

(event `self.ReceiveBeginPlay`
  (bind _returnvalue (`GameplayStatics.GetPlayerCameraManager` 0))
  (bind _returnvalue_2 (pcsubsystem `EnhancedInputLocalPlayerSubsystem` (`GameplayStatics.GetPlayerController` 0)))
  (`KismetSystemLibrary.PrintString` (`KismetStringLibrary.Conv_VectorToString` (`SceneComponent.K2_GetComponentLocation` (`self.Scene`))) true true (struct :`G` 0.66 :`B` 1.0 :`A` 1.0) 10.0)
  (`|ExecutionSequence`
    (:`then_0`
      ;[1 1 1] 检查本地增强输入是否有效，并添加增强输入
      (`/Engine/EditorBlueprintResources/StandardMacros.IsValid` _returnvalue_2
        (:`Is Valid`
          (`EnhancedInputSubsystemInterface.AddMappingContext` _returnvalue_2 "/Game/System/Character/Input/FPS_InputMappingContext.FPS_InputMappingContext" 0 (struct))
          ;[1 1 1] 设置俯仰角
          (set `PlayerCameraManager.ViewPitchMax` 80.0 _returnvalue)
          (set `PlayerCameraManager.ViewPitchMin` -80.0 _returnvalue)
          ;[1 1 1] 创建角色HUD
          (bind _returnvalue_3 (`|CreateWidget` "/Game/System/Character/BP/Player_HUD.Player_HUD_C"))
          (bind _output_get (set `self.HUD` _returnvalue_3))
          (`UserWidget.AddToViewport` _output_get 0)
          (bind _asplayer_abp (cast `/Game/System/Character/Animations/Player_ABP` (`SkeletalMeshComponent.GetAnimInstance` (`self.FPS_SKM`))))
          (set `self.As Player ABP` _asplayer_abp))
        (:`Is Not Valid`
          (`KismetSystemLibrary.PrintString` "增强输入本地玩家子系统无效！"))))
    (:`then_1`
      (`KismetSystemLibrary.K2_SetTimer` null "CameraAutoDOF" 0.2 true))))

(event `CameraAutoDOF`
  (bind _camera (`self.Camera`))
  (bind _camera_2 (`self.Camera`))
  (bind _returnvalue (`SceneComponent.K2_GetComponentLocation` _camera_2))
  ;[1 1 1] 相机自适应景深
  (bind (_outhit _returnvalue_2) (`KismetSystemLibrary.LineTraceSingle` _returnvalue (+ _returnvalue (* (`SceneComponent.GetForwardVector` _camera_2) 10000.0)) "TraceTypeQuery1"))
  (if _returnvalue_2
    (set `self.FocusLoc` (`KismetMathLibrary.VSize` (- (`.Location` (`GameplayStatics.BreakHitResult` _outhit)) (`SceneComponent.K2_GetComponentLocation` _camera))))
    (set `CameraComponent.PostProcessSettings` (make `PostProcessSettings` :`DepthOfFieldFstop` 25.0 :`DepthOfFieldMinFstop` 100.0 :`DepthOfFieldFocalDistance` (`self.FocusLoc`)) _camera)))

(event `CameraShake`
  (bind _returnvalue (`GameplayStatics.GetPlayerController` 0))
  ;[1 1 1] 镜头晃动
  (if (<= (`KismetMathLibrary.VSize` (`self.GetVelocity`)) 0.0)
    (`PlayerController.ClientStartCameraShake` :`self` _returnvalue :`Shake` "/Game/System/CameraShake/CameraShake_Idle.CameraShake_Idle_C")
    (elif (>= (`KismetMathLibrary.VSize` (`self.GetVelocity`)) 301.0)
      (`PlayerController.ClientStartCameraShake` :`self` _returnvalue :`Shake` "/Game/System/CameraShake/CameraShake_Run.CameraShake_Run_C")
      (else
        (`PlayerController.ClientStartCameraShake` :`self` _returnvalue :`Shake` "/Game/System/CameraShake/CameraShake_Walk.CameraShake_Walk_C")))))

(event `EnhancedInput|/Game/System/Character/Input/IA_Sprint`
  (params (ActionValue :type Boolean) (ElapsedSeconds :type "Float (double-precision)") (TriggeredSeconds :type "Float (double-precision)") (InputAction :type "InputAction Object Reference" :default "/Game/System/Character/Input/IA_Sprint.IA_Sprint"))
  (bind _e_playerstate (`self.E_PlayerState`))
  ;[1 1 1] 冲刺
  (:`Started`
    (switch `/Game/System/Enum/E_PlayerState` _e_playerstate
      (:`NewEnumerator0`
        (`self.SetMaxWalkSpeed` "NewEnumerator2"))))
  (:`Completed`
    (switch `/Game/System/Enum/E_PlayerState` _e_playerstate
      (:`NewEnumerator2`
        (`self.SetMaxWalkSpeed` "NewEnumerator0")))))

(event `EnhancedInput|/Game/System/Character/Input/IA_Move`
  (params (ActionValue :type "Vector2D Structure") (ElapsedSeconds :type "Float (double-precision)") (TriggeredSeconds :type "Float (double-precision)") (InputAction :type "InputAction Object Reference" :default "/Game/System/Character/Input/IA_Move.IA_Move"))
  (bind (_x _y) (`KismetMathLibrary.BreakVector2D` ActionValue))
  ;[1 1 1] 移动
  (:`Triggered`
    (`self.AddMovementInput` (`self.GetActorRightVector`) _x)
    (`self.RollSway` _x)
    (`self.AddMovementInput` (`self.GetActorForwardVector`) _y)))

(event `EnhancedInput|/Game/System/Character/Input/IA_Jump`
  (params (ActionValue :type Boolean) (ElapsedSeconds :type "Float (double-precision)") (TriggeredSeconds :type "Float (double-precision)") (InputAction :type "InputAction Object Reference" :default "/Game/System/Character/Input/IA_Jump.IA_Jump"))
  ;[1 1 1] 跳跃
  (:`Started`
    (switch `/Game/System/Enum/E_PlayerState` (`self.E_PlayerState`)
      (:`NewEnumerator0`
        (`self.Jump` :!label _label))
      (:`NewEnumerator3`
        ;[1 1 1] 蹲伏
        (bind _returnvalue (`self.CrouchObstacleDetection` :!label _label_2))
        (if (not _returnvalue)
          (`self.SetMaxWalkSpeed` "NewEnumerator0")
          (bind (_direction _lerp) (`Timeline|CrouchLerp` :!via `Reverse` :!label _label_3)
            (:`Update`
              (`CapsuleComponent.SetCapsuleHalfHeight` (`self.CapsuleComponent`) (`KismetMathLibrary.Lerp` 88.0 55.0 _lerp) true)))))
      (:`NewEnumerator2`
        (goto _label))))
  (:`Completed`
    (`self.StopJumping`)))

(event `EnhancedInput|/Game/System/Character/Input/IA_Look`
  (params (ActionValue :type "Vector2D Structure") (ElapsedSeconds :type "Float (double-precision)") (TriggeredSeconds :type "Float (double-precision)") (InputAction :type "InputAction Object Reference" :default "/Game/System/Character/Input/IA_Look.IA_Look"))
  ;[1 1 1] 查看
  (:`Triggered`
    (bind _output_get (set `self.Action Value` ActionValue))
    (bind (_x _y) (`KismetMathLibrary.BreakVector2D` _output_get))
    (`self.AddControllerYawInput` _x)
    (`self.YawSway` _x)
    (`self.AddControllerPitchInput` _y)
    (`self.PitchSway` _y)))

(event `EnhancedInput|/Game/System/Character/Input/IA_Crouch`
  (params (ActionValue :type Boolean) (ElapsedSeconds :type "Float (double-precision)") (TriggeredSeconds :type "Float (double-precision)") (InputAction :type "InputAction Object Reference" :default "/Game/System/Character/Input/IA_Crouch.IA_Crouch"))
  ;[1 1 1] 蹲伏
  (:`Started`
    (switch `/Game/System/Enum/E_PlayerState` (`self.E_PlayerState`)
      (:`NewEnumerator0`
        _)
      (:`NewEnumerator3`
        (goto _label_2))
      (:`NewEnumerator2`
        _))
    (`self.SetMaxWalkSpeed` "NewEnumerator3")
    (goto _label_3)))

(event `EnhancedInput|/Game/System/Character/Input/IA_SwitchWeapon_1`
  (params (ActionValue :type Boolean) (ElapsedSeconds :type "Float (double-precision)") (TriggeredSeconds :type "Float (double-precision)") (InputAction :type "InputAction Object Reference" :default "/Game/System/Character/Input/IA_SwitchWeapon_1.IA_SwitchWeapon_1"))
  ;[0.06771 0.03985 0.03985] （废案）拾取枪械
  ;;[0.06771 0.03985 0.03985] 注释
)

(event `EnhancedInput|/Game/System/Character/Input/IA_Grab`
  (params (ActionValue :type Boolean) (ElapsedSeconds :type "Float (double-precision)") (TriggeredSeconds :type "Float (double-precision)") (InputAction :type "InputAction Object Reference" :default "/Game/System/Character/Input/IA_Grab.IA_Grab"))
  ;[1 1 1] 拾取枪械
  (:`Started`
    (`self.InteractionHitActor`
      (:`then`
        (bind _weapondataasset (message `/Game/System/Character/BP/PickUp_BPI.GetDataAsset` (`self.InteractionHitActor`)))
        (bind _returnvalue (`|SpawnActorFromClass` (`/Game/System/DataAsset/Gun_DataAsset.GunClass` _weapondataasset) (`KismetMathLibrary.MakeTransform` (0.0 0.0 0.0)) "AlwaysSpawn" "MultiplyWithRoot" null _weapondataasset null))
        (switch `/Game/System/Enum/E_GunType` (`/Game/System/DataAsset/Gun_DataAsset.E_GunType` _weapondataasset)
          (:`NewEnumerator2`
            (bind _itemweapon_slot1 (`self.ItemWeapon_Slot1`)
              (:`then`
                (switch `/Game/System/Enum/E_GunType` (`self.HeldGunState`)
                  (:`NewEnumerator0`
                    (bind _gundataasset (`/Game/System/WeaponBP/GunBP/Item_Weapon_Gun.GunDataAsset` _itemweapon_slot1))
                    ;;[1 1 1] 如果捡起来的是手枪，则直接捡起并手持
                    (`self.DropGun` _gundataasset :!label _label)
                    (set `self.ItemWeapon_Slot1` _returnvalue)
                    (`self.SwitchWeaponSlot` :!label _label_2)
                    (set `self.HeldGunState` "NewEnumerator2"))
                  (:`NewEnumerator2`
                    ;;[0.6847 0.9601 1] 替换手中的1号槽的枪械
                    (`self.DropGun` _gundataasset)
                    (bind _output_get (set `self.ItemWeapon_Slot1` _returnvalue))
                    (`self.PutAway` _output_get))
                  (:`NewEnumerator1`
                    (goto _label))))
              (:`else`
                ;;[1 1 1] 1号步枪槽位没有枪械时，捡起直接手持
                (set `self.ItemWeapon_Slot1` _returnvalue)
                (goto _label_2))))
          (:`NewEnumerator1`
            (bind _itemweapon_slot2 (`self.ItemWeapon_Slot2`)
              (:`then`
                (switch `/Game/System/Enum/E_GunType` (`self.HeldGunState`)
                  (:`NewEnumerator0`
                    (bind _gundataasset_2 (`/Game/System/WeaponBP/GunBP/Item_Weapon_Gun.GunDataAsset` _itemweapon_slot2))
                    ;;[1 1 1] 如果捡起来的是步枪，则直接捡起并手持
                    (`self.DropGun` _gundataasset_2 :!label _label_3)
                    (set `self.ItemWeapon_Slot2` _returnvalue)
                    (`self.SwitchWeaponSlot` :!label _label_4)
                    (set `self.HeldGunState` "NewEnumerator1"))
                  (:`NewEnumerator2`
                    (goto _label_3))
                  (:`NewEnumerator1`
                    ;;[0.6652 0.9701 1] 替换手中的2号槽的枪械
                    (`self.DropGun` _gundataasset_2)
                    (bind _output_get_2 (set `self.ItemWeapon_Slot2` _returnvalue))
                    (`self.PutAway` _output_get_2))))
              (:`else`
                ;;[1 1 1] 2号手枪槽位没有枪械时，捡起直接手持
                (set `self.ItemWeapon_Slot2` _returnvalue)
                (goto _label_4)))))
        (`self.K2_DestroyActor` (`self.InteractionHitActor`))
        (set `self.InteractionHitActor` null))
      (:`else`))))

(event `EnhancedInput|/Game/System/Character/Input/IA_SwitchWeapon_2`
  (params (ActionValue :type Boolean) (ElapsedSeconds :type "Float (double-precision)") (TriggeredSeconds :type "Float (double-precision)") (InputAction :type "InputAction Object Reference" :default "/Game/System/Character/Input/IA_SwitchWeapon_2.IA_SwitchWeapon_2"))
  ;[0.06771 0.03985 0.03985] （废案）拾取枪械
  ;;[0.06771 0.03985 0.03985] 注释
)

(event `EnhancedInput|/Game/System/Character/Input/IA_Grab`
  (params (ActionValue :type Boolean) (ElapsedSeconds :type "Float (double-precision)") (TriggeredSeconds :type "Float (double-precision)") (InputAction :type "InputAction Object Reference" :default "/Game/System/Character/Input/IA_Grab.IA_Grab"))
  ;[0.06771 0.03985 0.03985] （废案）拾取枪械
)

(event `SwitchWeaponSlot`
  ;[1 1 1] 切换枪械
  (switch `/Game/System/Enum/E_GunType` (`self.HeldGunState`) :!label _label_5
    (:`NewEnumerator0`
      (`|ExecutionSequence`
        (:`then_0`
          (bind _itemweapon_slot2 (`self.ItemWeapon_Slot2` :!label _label_6)
            (:`then`
              (`self.PutAway` _itemweapon_slot2)
              (set `self.HeldGunState` "NewEnumerator1"))
            (:`else`)))
        (:`then_1`
          (bind _itemweapon_slot1 (`self.ItemWeapon_Slot1` :!label _label_7)
            (:`then`
              (`self.PutAway` _itemweapon_slot1)
              (set `self.HeldGunState` "NewEnumerator2"))
            (:`else`)))))
    (:`NewEnumerator2`
      (goto _label_6))
    (:`NewEnumerator1`
      (goto _label_7))))

(event `EnhancedInput|/Game/System/Character/Input/IA_SwitchWeaponSlot`
  (params (ActionValue :type Boolean) (ElapsedSeconds :type "Float (double-precision)") (TriggeredSeconds :type "Float (double-precision)") (InputAction :type "InputAction Object Reference" :default "/Game/System/Character/Input/IA_SwitchWeaponSlot.IA_SwitchWeaponSlot"))
  ;[1 1 1] 切换枪械
  (:`Started`
    (goto _label_5)))

(event `PutAway`
  (params (`目标` :type "Actor Object Reference"))
  ;[1 1 1] 收枪/举枪
  (bind (_direction `_新建轨道_0`) (`Timeline|PutAway_TL` :!via `PlayFromStart` :!label _label_8)
    (:`Update`
      (`SceneComponent.K2_SetRelativeLocation` (`self.FPS_SKM`) (`KismetMathLibrary.MakeVector` 0.0 0.0 (`KismetMathLibrary.Lerp` -167.0 -260.0 `_新建轨道_0`)) false false))
    (:`Finished`
      (switch `ETimelineDirection` _direction
        (:`Forward`
          (`self.AllWeaponPlacedOnTheBack`
            (:`then_2`
              (bind _returnvalue (`self.WeaponPlacedOnTheHand` `目标`))
              (if _returnvalue
                (bind _weapondataasset (message `/Game/System/Character/BP/Item_BPI.GetItemDataAsset` `目标`))
                (bind _output_get (set `/Game/System/DataAsset/Gun_DataAsset.GunName` (`/Game/System/DataAsset/Gun_DataAsset.GunName` _weapondataasset) _weapondataasset))
                (set `/Game/System/Character/Animations/Player_ABP.gunName` _output_get (`self.As Player ABP`))
                (`self.Equip`)))))))))

(event `Equip`
  ;[1 1 1] 收枪/举枪
  (goto _label_8 :!via `Reverse`))

(event `EnhancedInput|/Game/System/Character/Input/IA_Grab`
  (params (ActionValue :type Boolean) (ElapsedSeconds :type "Float (double-precision)") (TriggeredSeconds :type "Float (double-precision)") (InputAction :type "InputAction Object Reference" :default "/Game/System/Character/Input/IA_Grab.IA_Grab"))
  ;[1 1 1] 拾取枪械
)

(event `EnhancedInput|/Game/System/Character/Input/IA_Fire`
  (params (ActionValue :type Boolean) (ElapsedSeconds :type "Float (double-precision)") (TriggeredSeconds :type "Float (double-precision)") (InputAction :type "InputAction Object Reference" :default "/Game/System/Character/Input/IA_Fire.IA_Fire"))
  (bind _itemweapon_slot1 (`self.ItemWeapon_Slot1`))
  (bind _itemweapon_slot2 (`self.ItemWeapon_Slot2`))
  (:`Started`
    (switch `/Game/System/Enum/E_GunType` (`self.HeldGunState`)
      (:`NewEnumerator2`
        (message `/Game/System/Character/BP/Item_BPI.Fire` _itemweapon_slot1)
        (set `self.ArmsMontage` (`/Game/System/WeaponBP/GunBP/Item_Weapon_Gun.ArmsFireMontage` _itemweapon_slot1)))
      (:`NewEnumerator1`
        (message `/Game/System/Character/BP/Item_BPI.Fire` _itemweapon_slot2)
        (set `self.ArmsMontage` (`/Game/System/WeaponBP/GunBP/Item_Weapon_Gun.ArmsFireMontage` _itemweapon_slot2))))
    (`|PlayMontage` (`self.FPS_SKM`) (`self.ArmsMontage`))))

(fn `PitchSway`
  (params (Value :type "Float (double-precision)"))
  (bind _root (`self.Root`))
  (bind (_weaponrotator_roll _weaponrotator_pitch) (`KismetMathLibrary.BreakRotator` (`self.WeaponRotator`)))
  (bind _relativerotation (`SceneComponent.RelativeRotation` _root))
  (`SceneComponent.K2_SetRelativeRotation` _root (`KismetMathLibrary.MakeRotator` (.roll _relativerotation) (`KismetMathLibrary.FInterpTo` _weaponrotator_pitch (* (`KismetMathLibrary.FClamp` Value -1.0) -3.0) (`GameplayStatics.GetWorldDeltaSeconds`) 5.0) (.yaw _relativerotation)) false false)
  (set `self.WeaponRotator` _relativerotation))

(fn `RollSway`
  (params (Value :type "Float (double-precision)"))
  (bind _root (`self.Root`))
  (bind _weaponrotator_roll (`KismetMathLibrary.BreakRotator` (`self.WeaponRotator`)))
  (bind _relativerotation (`SceneComponent.RelativeRotation` _root))
  (`SceneComponent.K2_SetRelativeRotation` _root (`KismetMathLibrary.MakeRotator` (`KismetMathLibrary.FInterpTo` _weaponrotator_roll (* (`KismetMathLibrary.FClamp` Value -1.0) 20.0) (`GameplayStatics.GetWorldDeltaSeconds`) 2.0) (.pitch _relativerotation) (.yaw _relativerotation)) false false)
  (set `self.WeaponRotator` _relativerotation))

(fn `UserConstructionScript`)

(fn `YawSway`
  (params (Value :type "Float (double-precision)"))
  (bind _root (`self.Root`))
  (bind (_weaponrotator_roll _weaponrotator_pitch _weaponrotator_yaw) (`KismetMathLibrary.BreakRotator` (`self.WeaponRotator`)))
  (bind _relativerotation (`SceneComponent.RelativeRotation` _root))
  (`SceneComponent.K2_SetRelativeRotation` _root (`KismetMathLibrary.MakeRotator` (.roll _relativerotation) (.pitch _relativerotation) (`KismetMathLibrary.FInterpTo` _weaponrotator_yaw (* (`KismetMathLibrary.FClamp` Value -1.0) 1.0) (`GameplayStatics.GetWorldDeltaSeconds`) 1.0)) false false)
  (set `self.WeaponRotator` _relativerotation))