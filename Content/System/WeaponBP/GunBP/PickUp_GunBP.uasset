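; PickUp_GunBP is a gun pickup that lies in the world as a physics-simulated static mesh.
; Its construction script takes the mesh from GunDataAsset, which GetDataAsset returns to callers.
; HighLight and CloseHighLight events set and clear an Interaction overlay material on the mesh to show or hide a highlight.
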(event `self.ReceiveBeginPlay`
  (`PrimitiveComponent.SetSimulatePhysics` (`self.StaticMesh`) true))

(event `/Game/System/Character/BP/PickUp_BPI.HighLight`
  (`MeshComponent.SetOverlayMaterial` (`self.StaticMesh`) "/Game/Resource/Material/Interaction.Interaction"))

(event `/Game/System/Character/BP/PickUp_BPI.CloseHighLight`
  (`MeshComponent.SetOverlayMaterial` (`self.StaticMesh`) null))

(fn `GetDataAsset`
  (returns (WeaponDataAsset :type "/Game/System/DataAsset/Gun_DataAsset Object Reference"))
  (return (`self.GunDataAsset`)))

(fn `UserConstructionScript`
  (`StaticMeshComponent.SetStaticMesh` (`self.StaticMesh`) (`/Game/System/DataAsset/Gun_DataAsset.GunSTM` (`self.GunDataAsset`))))